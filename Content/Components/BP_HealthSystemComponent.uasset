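; BP_HealthSystemComponent is an actor component that tracks its owner's health.
; It starts at max health and binds to the owner's OnTakeAnyDamage, clamping health, playing optional sound and Niagara effects, and broadcasting damage and death events.
; A Healed event adds HealthHealed with matching effects, but broadcasts only if health remains below max.
; The Kill and Heal functions are empty stubs.
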(event `self.ReceiveBeginPlay`
  (set `self.Owner` (`self.GetOwner`))
  (set `self.Health` (`self.MaxHealth`))
  (add `Actor.OnTakeAnyDamage` (`self.Owner`) (`|CreateDelegate` :!event `TookDamage`)))

(event `TookDamage`
  (params (DamagedActor :type "Actor Object Reference") (Damage :type "Float (single-precision)") (DamageType :type "DamageType Object Reference") (InstigatedBy :type "Controller Object Reference") (DamageCauser :type "Actor Object Reference"))
  (set `self.Health` (`KismetMathLibrary.FClamp` (- (`self.Health`) Damage) 0.0 (`self.MaxHealth`)))
  (`self.PlayFx`)
  (`self.OnTookDamage` Damage)
  (if (<= (`self.Health`) 0.0)
    (`self.OnKilled`)))

(event `Healed`
  (set `self.Health` (`KismetMathLibrary.FClamp` (+ (`self.Health`) (`self.HealthHealed`)) 0.0 (`self.MaxHealth`)))
  (`self.PlayHealFX`)
  (if (< (`self.Health`) (`self.MaxHealth`))
    (`self.OnHealed`)))

(fn `Heal`
  (params (HealthRecovered :type "Float (double-precision)")))

(fn `Kill`)

(fn `PlayFx`
  (bind _damagedsound (`self.DamagedSound`))
  (bind _damagedparticles (`self.DamagedParticles`))
  (`/Engine/EditorBlueprintResources/StandardMacros.IsValid` _damagedsound
    (:`Is Valid`
      (`GameplayStatics.PlaySoundAtLocation` _damagedsound (`Actor.K2_GetActorLocation` (`self.Owner`)) (struct) 1.0 1.0 0.0 null null null null))
    (:`Is Not Valid`
      _))
  (`/Engine/EditorBlueprintResources/StandardMacros.IsValid` _damagedparticles
    (:`Is Valid`
      (`NiagaraFunctionLibrary.SpawnSystemAtLocation` _damagedparticles (`Actor.K2_GetActorLocation` (`self.Owner`))))))

(fn `PlayHealFX`
  (bind _healedparticles (`self.HealedParticles`))
  (bind _healedsound (`self.HealedSound`))
  (`/Engine/EditorBlueprintResources/StandardMacros.IsValid` _healedsound
    (:`Is Valid`
      (`GameplayStatics.PlaySoundAtLocation` _healedsound (`Actor.K2_GetActorLocation` (`self.Owner`)) (struct) 1.0 1.0 0.0 null null null null))
    (:`Is Not Valid`
      _))
  (`/Engine/EditorBlueprintResources/StandardMacros.IsValid` _healedparticles
    (:`Is Valid`
      (`NiagaraFunctionLibrary.SpawnSystemAtLocation` _healedparticles (`Actor.K2_GetActorLocation` (`self.Owner`))))))