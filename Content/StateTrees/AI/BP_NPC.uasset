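; BP_NPC is an enemy actor that counts toward the game mode's EnemiesLeft tally and damages the player on contact.
; It increments that tally on BeginPlay, then decrements it and destroys itself when its health component reports OnKilled.
; Any Box overlap applies PlayerDamage to player 0's health component without checking the overlapping actor.
; The trailing three-second Delay leads to nothing, so it does not throttle damage.
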(event `self.ReceiveBeginPlay`
  (bind _asbp_first_person_game_mode (cast `/Game/FirstPerson/Blueprints/BP_FirstPersonGameMode` (`GameplayStatics.GetGameMode`)))
  (set `/Game/FirstPerson/Blueprints/BP_FirstPersonGameMode.Enemies Left` (+ (`/Game/FirstPerson/Blueprints/BP_FirstPersonGameMode.Enemies Left` _asbp_first_person_game_mode) 1) _asbp_first_person_game_mode)
  (add `/Game/Components/BP_HealthSystemComponent.OnKilled` (`self.BP_HealthSystemComponent`) (delegate `OnKilled`)))

(event `OnKilled`
  (bind _asbp_first_person_game_mode (cast `/Game/FirstPerson/Blueprints/BP_FirstPersonGameMode` (`GameplayStatics.GetGameMode`)))
  (set `/Game/FirstPerson/Blueprints/BP_FirstPersonGameMode.Enemies Left` (- (`/Game/FirstPerson/Blueprints/BP_FirstPersonGameMode.Enemies Left` _asbp_first_person_game_mode) 1) _asbp_first_person_game_mode)
  (`self.K2_DestroyActor`))

(event `self.Box.OnComponentBeginOverlap`
  (params (OverlappedComponent :type "PrimitiveComponent Object Reference") (OtherActor :type "Actor Object Reference") (OtherComp :type "PrimitiveComponent Object Reference") (OtherBodyIndex :type Integer) (bFromSweep :type Boolean) (SweepResult :type "HitResult Structure (by ref)"))
  (bind _returnvalue (`self.GetComponentByClass` (`GameplayStatics.GetPlayerPawn` 0) "/Game/Components/BP_HealthSystemComponent.BP_HealthSystemComponent_C"))
  (`/Engine/EditorBlueprintResources/StandardMacros.IsValid` _returnvalue
    (:`Is Valid`
      (`/Game/Components/BP_HealthSystemComponent.TookDamage` _returnvalue (`GameplayStatics.GetPlayerPawn` 0) (`self.PlayerDamage`) null null null)
      (`KismetSystemLibrary.Delay` 3.0))))

(fn `UserConstructionScript`)