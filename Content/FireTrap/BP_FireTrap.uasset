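; Fire trap actor that warms up when a character touches its activation volume, then burns the player for a timed period.
; An enum state machine with enter/exit functions cycles Idle, Warming and Hot on timers, swapping particles and sounds.
; The touch dispatcher is bound only in Idle, and the damage volume, active only when Hot, damages the player's BP_HealthSystemComponent on overlap.
; Disabled shuts off activation and has no outgoing transition.
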(event `self.ReceiveBeginPlay`
  (`PrimitiveComponent.SetCollisionEnabled` (`self.DamageVolume`) "NoCollision")
  (`self.ChangeState` "NewEnumerator0"))

(event `self.ReceiveTick`
  (params (DeltaSeconds :type "Float (single-precision)"))
  (switch `/Game/FireTrap/E_FireTrapState` (`self.CurrentState`)))

(event `self.ActivateVolume.OnComponentBeginOverlap`
  (params (OverlappedComponent :type "PrimitiveComponent Object Reference") (OtherActor :type "Actor Object Reference") (OtherComp :type "PrimitiveComponent Object Reference") (OtherBodyIndex :type Integer) (bFromSweep :type Boolean) (SweepResult :type "HitResult Structure (by ref)"))
  (cast `Character` OtherActor)
  (`self.OnTrapTouched`))

(event `self.DamageVolume.OnComponentBeginOverlap`
  (params (OverlappedComponent :type "PrimitiveComponent Object Reference") (OtherActor :type "Actor Object Reference") (OtherComp :type "PrimitiveComponent Object Reference") (OtherBodyIndex :type Integer) (bFromSweep :type Boolean) (SweepResult :type "HitResult Structure (by ref)"))
  (if (== OtherActor (`GameplayStatics.GetPlayerPawn` 0))
    (`/Game/Components/BP_HealthSystemComponent.TookDamage` (`self.GetComponentByClass` (`GameplayStatics.GetPlayerPawn` 0) "/Game/Components/BP_HealthSystemComponent.BP_HealthSystemComponent_C") (`GameplayStatics.GetPlayerPawn` 0) (`self.Player Damage`) null null null)
    (`KismetSystemLibrary.Delay` 3.0)))

(fn `ActivateTrap`
  (`self.ChangeState` "NewEnumerator1"))

(fn `ChangeState`
  (params (NewState :type "/Game/FireTrap/E_FireTrapState Enum" :default "NewEnumerator0"))
  (if (`self.IsInitialState`)
    (set `self.IsInitialState` false)
    (set `self.CurrentState` NewState :!label _label)
    (switch `/Game/FireTrap/E_FireTrapState` (`self.CurrentState`)
      (:`NewEnumerator0`
        (`self.EnterIdleState`))
      (:`NewEnumerator1`
        (`self.EnterWarmingState`))
      (:`NewEnumerator2`
        (`self.EnterHotState`))
      (:`NewEnumerator3`
        (`self.EnterDisabledState`)))
    (elif (not (`|EnumEquality` NewState (`self.CurrentState`)))
      (switch `/Game/FireTrap/E_FireTrapState` (`self.CurrentState`)
        (:`NewEnumerator0`
          (`self.ExitIdleState`)
          (goto _label))
        (:`NewEnumerator1`
          (`self.ExitWarmingState`)
          (goto _label))
        (:`NewEnumerator2`
          (`self.ExitHotState`)
          (goto _label))))))

(fn `EnterDisabledState`
  (bind _trapparticles (`self.TrapParticles`))
  (`PrimitiveComponent.SetCollisionEnabled` (`self.ActivateVolume`) "NoCollision")
  (`GameplayStatics.PlaySoundAtLocation` (`self.DisabledSound`) (`self.K2_GetActorLocation`) (struct) 1.0 1.0 0.0 null null null null)
  (`NiagaraComponent.SetAsset` _trapparticles (`self.DisabledParticles`) true)
  (`ActorComponent.Activate` _trapparticles false))

(fn `EnterHotState`
  (bind _trapparticles (`self.TrapParticles`))
  (bind _trapaudio (`self.TrapAudio`))
  (`PrimitiveComponent.SetCollisionEnabled` (`self.DamageVolume`) "QueryAndPhysics")
  (`NiagaraComponent.SetAsset` _trapparticles (`self.HotParticles`) true)
  (`ActorComponent.Activate` _trapparticles false)
  (`AudioComponent.SetSound` _trapaudio (`self.HotLoopingSound`))
  (`ActorComponent.Activate` _trapaudio false)
  (`GameplayStatics.PlaySoundAtLocation` (`self.HotActivateSound`) (`self.K2_GetActorLocation`) (struct) 1.0 1.0 0.0 null null null null)
  (`KismetSystemLibrary.K2_SetTimer` null "OnHotTimerEnded" (`self.HotDuration`)))

(fn `EnterIdleState`
  (add `self.OnTrapTouched` (`|CreateDelegate` :!event `ActivateTrap`)))

(fn `EnterWarmingState`
  (bind _trapparticles (`self.TrapParticles`))
  (`NiagaraComponent.SetAsset` _trapparticles (`self.WarmingParticles`) true)
  (`ActorComponent.Activate` _trapparticles false)
  (`GameplayStatics.PlaySoundAtLocation` (`self.ActivateWarmingSound`) (`self.K2_GetActorLocation`) (struct) 1.0 1.0 0.0 null null null null)
  (`KismetSystemLibrary.K2_SetTimer` null "OnWarmingTimerEnded" (`self.WarmingDuration`)))

(fn `ExitDisableState`)

(fn `ExitHotState`
  (`PrimitiveComponent.SetCollisionEnabled` (`self.DamageVolume`) "NoCollision")
  (`ActorComponent.Deactivate` (`self.TrapParticles`))
  (`ActorComponent.Deactivate` (`self.TrapAudio`)))

(fn `ExitIdleState`
  (remove `self.OnTrapTouched` (`|CreateDelegate` :!event `ActivateTrap`)))

(fn `ExitWarmingState`
  (`ActorComponent.Deactivate` (`self.TrapParticles`)))

(fn `OnHotTimerEnded`
  (`self.ChangeState` "NewEnumerator0"))

(fn `OnWarmingTimerEnded`
  (`self.ChangeState` "NewEnumerator2"))

(fn `TickDisableState`)

(fn `TickHotState`)

(fn `TickIdleState`)

(fn `TickWarmingState`)

(fn `UserConstructionScript`)