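; BP_TrapSwitch is an interactable switch that changes the state of a fire trap.
; On StartInteract, it casts its fire trap reference to BP_FireTrap, looks up an actor with GetActorOfClass, and calls ChangeState with one fixed enum value.
; The class lookup returns the first matching actor in the level, and the switch has no toggle or other active logic.
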(event `self.StartInteract`
  (bind _asbp_fire_trap (castclass `/Game/FireTrap/BP_FireTrap` "/Game/FireTrap/BP_FireTrap.BP_FireTrap_C"))
  (bind _returnvalue (`GameplayStatics.GetActorOfClass` _asbp_fire_trap))
  (`/Game/FireTrap/BP_FireTrap.ChangeState` _returnvalue "NewEnumerator3"))

(fn `UserConstructionScript`
  (`parent.UserConstructionScript`))