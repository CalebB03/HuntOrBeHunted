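; BP_HealthPickup is a health pickup actor that heals the player when a shooter character touches it.
; Its sphere collision overlap accepts only BP_ShooterCharacter and continues only if that character's health is below maximum.
; It then calls Healed on the health system component of player pawn 0, rather than the overlapping character, and destroys itself.
; The heal amount is left to that component.
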(event `self.Sphere Collision.OnComponentBeginOverlap`
  (params (OverlappedComponent :type "PrimitiveComponent Object Reference") (OtherActor :type "Actor Object Reference") (OtherComp :type "PrimitiveComponent Object Reference") (OtherBodyIndex :type Integer) (bFromSweep :type Boolean) (SweepResult :type "HitResult Structure (by ref)"))
  (bind _returnvalue (`self.GetComponentByClass` (`GameplayStatics.GetPlayerPawn` 0) "/Game/Components/BP_HealthSystemComponent.BP_HealthSystemComponent_C"))
  (bind _asbp_shooter_character (cast `/Game/Variant_Shooter/Blueprints/BP_ShooterCharacter` OtherActor))
  (bind _bp_healthsystemcomponent (`/Game/Variant_Shooter/Blueprints/BP_ShooterCharacter.BP_HealthSystemComponent` _asbp_shooter_character))
  (if (< (`/Game/Components/BP_HealthSystemComponent.Health` _bp_healthsystemcomponent) (`/Game/Components/BP_HealthSystemComponent.MaxHealth` _bp_healthsystemcomponent))
    (`/Engine/EditorBlueprintResources/StandardMacros.IsValid` _returnvalue
      (:`Is Valid`
        (`/Game/Components/BP_HealthSystemComponent.Healed` _returnvalue)
        (`self.K2_DestroyActor`)))))

(fn `UserConstructionScript`
  (`parent.UserConstructionScript`))