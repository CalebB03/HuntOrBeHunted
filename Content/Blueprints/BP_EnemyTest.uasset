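; BP_EnemyTest is a test enemy actor that damages the player through an overlap box and is destroyed when killed.
; On BeginPlay it binds to the killed event of its health system component, which triggers DestroyActor.
; Any box overlap applies PlayerDamage to player pawn 0 through that pawn's health component, without checking which actor overlapped.
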(event `self.ReceiveBeginPlay`
  (add `/Game/Components/BP_HealthSystemComponent.OnKilled` (`self.BP_HealthSystemComponent`) (delegate `OnKilled`)))

(event `OnKilled`
  (`self.K2_DestroyActor`))

(event `self.Box.OnComponentBeginOverlap`
  (params (OverlappedComponent :type "PrimitiveComponent Object Reference") (OtherActor :type "Actor Object Reference") (OtherComp :type "PrimitiveComponent Object Reference") (OtherBodyIndex :type Integer) (bFromSweep :type Boolean) (SweepResult :type "HitResult Structure (by ref)"))
  (bind _returnvalue (`self.GetComponentByClass` (`GameplayStatics.GetPlayerPawn` 0) "/Game/Components/BP_HealthSystemComponent.BP_HealthSystemComponent_C"))
  (`/Engine/EditorBlueprintResources/StandardMacros.IsValid` _returnvalue
    (:`Is Valid`
      (`/Game/Components/BP_HealthSystemComponent.TookDamage` _returnvalue (`GameplayStatics.GetPlayerPawn` 0) (`self.PlayerDamage`) null null null))))

(fn `UserConstructionScript`)