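; Base pickup actor that triggers when the first player's pawn overlaps its sphere collision.
; On overlap it runs PlayFX, calls the Pickup event, then destroys itself.
; PlayFX plays an optional sound and spawns an optional Niagara effect at the actor's location.
; Pickup is empty here, serving as the hook for child Blueprints to define the pickup's effect.
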(event `self.Sphere Collision.OnComponentBeginOverlap`
  (params (OverlappedComponent :type "PrimitiveComponent Object Reference") (OtherActor :type "Actor Object Reference") (OtherComp :type "PrimitiveComponent Object Reference") (OtherBodyIndex :type Integer) (bFromSweep :type Boolean) (SweepResult :type "HitResult Structure (by ref)"))
  (if (== OtherActor (`GameplayStatics.GetPlayerPawn` 0))
    (`self.PlayFX`)
    (`self.Pickup` null)
    (`self.K2_DestroyActor`)))

(event `Pickup`
  (params (PlayerPawn :type "Pawn Object Reference")))

(fn `PlayFX`
  (bind _pickupsound (`self.PickupSound`))
  (bind _pickupparticles (`self.PickupParticles`))
  (`/Engine/EditorBlueprintResources/StandardMacros.IsValid` _pickupsound
    (:`Is Valid`
      (`GameplayStatics.PlaySoundAtLocation` _pickupsound (`self.K2_GetActorLocation`) (struct) 1.0 1.0 0.0 null null null null))
    (:`Is Not Valid`
      _))
  (`/Engine/EditorBlueprintResources/StandardMacros.IsValid` _pickupparticles
    (:`Is Valid`
      (`NiagaraFunctionLibrary.SpawnSystemAtLocation` _pickupparticles (`self.K2_GetActorLocation`)))
    (:`Is Not Valid`
      _))
  (return))

(fn `UserConstructionScript`)