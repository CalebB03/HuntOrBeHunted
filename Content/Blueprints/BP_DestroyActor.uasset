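; BP_DestroyActor is an interactable actor that removes itself with a splatter effect when interacted with.
; StartInteract calls DestroyActor first, then plays the Splatter_Cue sound and spawns the BP_DamageBurst Niagara system at the actor's location.
; BeginPlay, overlap and Tick are disabled stubs, and the construction script only calls its parent.
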(event `/Game/Blueprints/BPI_Interact.StartInteract`
  (`self.K2_DestroyActor`)
  (`GameplayStatics.PlaySoundAtLocation` "/Game/Sounds/Splatter_Cue.Splatter_Cue" (`self.K2_GetActorLocation`) (struct) 1.0 1.0 0.0 null null null null)
  (`NiagaraFunctionLibrary.SpawnSystemAtLocation` "/Game/FX/BP_DamageBurst.BP_DamageBurst" (`self.K2_GetActorLocation`)))

(fn `UserConstructionScript`
  (`parent.UserConstructionScript`))